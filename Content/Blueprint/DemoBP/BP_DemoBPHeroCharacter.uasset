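; Demo hero character Blueprint that configures its own components at runtime for a fixed, angled follow camera.
; Possession caches the controller, and BeginPlay runs the setup only if that controller is valid, also making the actor tickable while paused.
; Chained sequences configure a very thin capsule, hero mesh with AnimBP and material, lag-free collisionless spring arm with absolute rotation, and acceleration-based requested movement.
; Connect and disconnect events only toggle a Connected flag.
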(event Custom|InitAllComponents
  (bind _capsulecomponent (Variables|Default|GetCapsuleComponent))
  (bind _mesh (Variables|Character|GetMesh))
  (bind _springarm (Variables|Default|GetSpringArm))
  ;[1 1 1] Init components
  (Class|Actor|SetTickablewhenPaused true)
  ;;[1 0.6917 0.6297] capsule
  (Utilities|FlowControl|Sequence
    (:then_0
      (Components|Capsule|SetCapsuleHalfHeight _capsulecomponent 75.0 true))
    (:then_1
      (Components|Capsule|SetCapsuleRadius _capsulecomponent 1.0 true)
      ;;[1 0.6917 0.6297] mesh
      (Utilities|FlowControl|Sequence
        (:then_0
          (Class|SkinnedMeshComponent|SetSkeletalMesh _mesh "/Game/Blender/mc3.mc3_Body7" true))
        (:then_1
          (Transformation|SetRelativeTransform _mesh (Variables|Default|GetMeshTransform) false false))
        (:then_2
          (Class|SkeletalMeshComponent|SetAnimClass _mesh "/Game/Blueprint/DemoBP/ABP_DemoBP.ABP_DemoBP_C"))
        (:then_3
          (Rendering|Material|SetMaterial _mesh 0 "/Game/Materials/M_Hero.M_Hero")
          ;;[1 0.6917 0.6297] spring arm
          (Utilities|FlowControl|Sequence
            (:then_0
              (Variables|/Script/Engine.SpringArmComponent|SetTargetArmLength _springarm 1e+03))
            (:then_1
              (Variables|/Script/Engine.SpringArmComponent|SetbDoCollisionTest _springarm false))
            (:then_2
              (Variables|/Script/Engine.SpringArmComponent|SetbEnableCameraLag _springarm false))
            (:then_3
              (Variables|/Script/Engine.SpringArmComponent|SetCameraLagSpeed _springarm 2e+01))
            (:then_4
              (Transformation|SetAbsolute _springarm false true false))
            (:then_5
              (Transformation|SetRelativeTransform _springarm (Math|Transform|MakeTransform "0, 0, 0" "-45.000000, 0, 0") false false)
              ;;[1 0.6917 0.6297] movement
              (Utilities|FlowControl|Sequence
                (:then_0
                  (Variables|/Script/Engine.CharacterMovementComponent|SetbRequestedMoveUseAcceleration (Variables|Character|GetCharacterMovement) true))))))))))

(event Custom|OnConnected
  (Variables|Default|SetbConnected true))

(event Custom|OnDisconnected
  (Variables|Default|SetbConnected false))

(event EventBeginPlay
  (Utilities|IsValid (Variables|Default|GetCachedPlayerController)
    (:Is%20Valid
      (CallFunction|InitAllComponents))))

(event EventTick
  (params (DeltaSeconds :type Float%20%28single-precision%29)))

(event EventPossessed
  (params (NewController :type Controller%20Object%20Reference))
  (Variables|Default|SetCachedPlayerController NewController))

(fn ConstructionScript
  (|CallParentFunction))