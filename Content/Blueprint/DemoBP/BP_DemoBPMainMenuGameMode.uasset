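; Main menu game mode that handles player login for the DemoBP demo.
; Login builds a JSON credentials string and sends it through the game instance's JSON-RPC client, showing a loading screen or an error.
; The OnLogin callback checks the returned username, caches user info and online state on the game instance, then opens the DemoBP level after a short delay.
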(event Custom|Login
  (params (Password :type String) (UserName :type String))
  (bind _asbp_demo_bpgame_instance (Utilities|Casting|CastToBP_DemoBPGameInstance (Game|GetGameInstance)))
  (bind _output_get (Variables|Default|SetCached%20Game%20Instance _asbp_demo_bpgame_instance))
  (Utilities|IsValid (Variables|/Game/Blueprint/DemoBP/BP_DemoBPGameInstance.BP_DemoBPGameInstance_C|GetJsonRpcClient _output_get)
    (:Is%20Valid
      (Variables|Default|SetCached%20Json%20Rpc%20Client (Variables|/Game/Blueprint/DemoBP/BP_DemoBPGameInstance.BP_DemoBPGameInstance_C|GetJsonRpcClient _output_get))
      (bind _jsonmsg (Utilities|NewLoginRequest Password UserName)
        (:Out
          (bind _returnvalue (Class|ERpcConnection|Request (Variables|Default|GetCached%20Json%20Rpc%20Client) "Login" _jsonmsg (delegate Custom|OnLogin) 10))
          (if (.bOk (Utilities|Struct|BreakERpcError _returnvalue))
            (Default|ShowLoadingScreen (Variables|Default|GetCached%20Game%20Instance) "正在加载地图...")
            (else
              (Default|ShowError (Variables|Default|GetCached%20Game%20Instance) (.Message (Utilities|Struct|BreakERpcError _returnvalue))))))))))

(event Custom|OnLogin
  (params (Connection :type E%20Rpc%20Connection%20Object%20Reference) (Response :type String) (RpcError :type E%20Rpc%20Error%20Structure))
  (bind (_bok _message) (Utilities|Struct|BreakERpcError RpcError))
  (bind _cached_game_instance (Variables|Default|GetCached%20Game%20Instance))
  (if _bok
    (bind _output_get (Variables|Default|SetLoginResponse (Class|EjsonValue|MakeJsonfromString Response)))
    (Utilities|IsValid (Class|EjsonValue|GetFieldValue _output_get "username")
      (:Is%20Valid
        (if (Utilities|Enum|Equal(Enum) (.Value (Class|EjsonValue|JsonasString (Class|EjsonValue|GetFieldValue _output_get "username"))) (stale Custom|Login UserName))
          (Variables|/Game/Blueprint/DemoBP/BP_DemoBPGameInstance.BP_DemoBPGameInstance_C|SetCachedUserInfo _cached_game_instance (Variables|Default|GetLoginResponse))
          (Variables|/Game/Blueprint/DemoBP/BP_DemoBPGameInstance.BP_DemoBPGameInstance_C|SetbUserOnline _cached_game_instance true)
          (Utilities|FlowControl|Delay 1.0)
          (Game|OpenLevel(byName) "DemoBP")
          (else
            (Default|ShowError (Variables|Default|GetCached%20Game%20Instance) "bad username")))))
    (else
      (Default|ShowError (Variables|Default|GetCached%20Game%20Instance) _message))))

(fn ConstructionScript
  (|CallParentFunction))