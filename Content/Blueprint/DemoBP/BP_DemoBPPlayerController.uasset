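; Player controller for the demo hero that handles world-axis movement, cursor-facing rotation and multiplayer position sync over JSON-RPC.
; Tick smoothly turns the hero toward the cursor hit and sends its transform and velocity via UpdateLocation, throttled by a looping timer and one request in flight.
; Each response updates a username-keyed map, spawns BP_DemoBPProxyCharacter actors for new players and passes target transforms and velocities to all proxies.
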(event Custom|SetMouseDirection
  (bind _hitresult (Game|Player|GetHitResultUnderCursorbyChannel "TraceTypeQuery1" false))
  (bind (_bblockinghit _binitialoverlap _time _distance _location) (Collision|BreakHitResult _hitresult))
  ;[1 1 1] Input
  ;;[1 0.6917 0.6297] rotate
  (Utilities|IsValid (Variables|Default|GetCachedHero)
    (:Is%20Valid
      (if _bblockinghit
        (Variables|Default|SetMouseDirection (Math|Rotator|FindLookatRotation (* (Transformation|GetActorLocation (Variables|Default|GetCachedHero)) "1.000000,1.000000, 0") (* _location "1.000000,1.000000, 0")))))))

(event Custom|NewPlayerOnline
  (params (Username :type String))
  (bind _returnvalue (Game|SpawnActorfromClass "/Game/Blueprint/DemoBP/BP_DemoBPProxyCharacter.BP_DemoBPProxyCharacter_C" (Math|Transform|MakeTransform "500.000000,300.000000,300.000000") "Undefined" 0 0))
  (Variables|/Game/Blueprint/DemoBP/BP_DemoBPProxyCharacter.BP_DemoBPProxyCharacter_C|SetUsername _returnvalue Username))

(event Custom|OnUpdateLocation
  (params (Connection :type E%20Rpc%20Connection%20Object%20Reference) (Response :type String) (RpcError :type E%20Rpc%20Error%20Structure))
  (bind _returnvalue (Class|EjsonValue|MakeJsonfromString Response))
  (bind _returnvalue_2 (Class|EjsonValue|GetFieldValue _returnvalue "locations"))
  (bind _returnvalue_3 (Class|EjsonValue|GetFieldValue _returnvalue "playerlist"))
  (Variables|Default|SetbCanRequest true)
  (if (and (Utilities|IsValid _returnvalue_3) (Utilities|IsValid _returnvalue_2))
    (Variables|Default|SetTmpPlayerList _returnvalue_3)
    (Variables|Default|SetTmpLocations _returnvalue_2)
    (for (_array_element _array_index) (.Value (Class|EjsonValue|JsonasArray (Variables|Default|GetTmpPlayerList)))
      (if (Utilities|Map|Contains (Variables|Default|GetProxyCharacters) (.Value (Class|EjsonValue|JsonasString _array_element)))
        _
        (else
          (CallFunction|NewPlayerOnline (.Value (Class|EjsonValue|JsonasString _array_element)))))
      (Utilities|FlowControl|Sequence
        (:then_0
          (bind _val (CallFunction|GetValue (.Value (Utilities|Map|Find (.Value (Class|EjsonValue|JsonasObject (Utilities|Array|Get(acopy) (.Value (Class|EjsonValue|JsonasArray (Variables|Default|GetTmpLocations))) _array_index))) "x")))))
        (:then_1
          (bind _val_2 (CallFunction|GetValue (.Value (Utilities|Map|Find (.Value (Class|EjsonValue|JsonasObject (Utilities|Array|Get(acopy) (.Value (Class|EjsonValue|JsonasArray (Variables|Default|GetTmpLocations))) _array_index))) "y")))))
        (:then_2
          (bind _val_3 (CallFunction|GetValue (.Value (Utilities|Map|Find (.Value (Class|EjsonValue|JsonasObject (Utilities|Array|Get(acopy) (.Value (Class|EjsonValue|JsonasArray (Variables|Default|GetTmpLocations))) _array_index))) "z")))))
        (:then_3
          (bind _val_4 (CallFunction|GetValue (.Value (Utilities|Map|Find (.Value (Class|EjsonValue|JsonasObject (Utilities|Array|Get(acopy) (.Value (Class|EjsonValue|JsonasArray (Variables|Default|GetTmpLocations))) _array_index))) "roll")))))
        (:then_4
          (bind _val_5 (CallFunction|GetValue (.Value (Utilities|Map|Find (.Value (Class|EjsonValue|JsonasObject (Utilities|Array|Get(acopy) (.Value (Class|EjsonValue|JsonasArray (Variables|Default|GetTmpLocations))) _array_index))) "pitch")))))
        (:then_5
          (bind _val_6 (CallFunction|GetValue (.Value (Utilities|Map|Find (.Value (Class|EjsonValue|JsonasObject (Utilities|Array|Get(acopy) (.Value (Class|EjsonValue|JsonasArray (Variables|Default|GetTmpLocations))) _array_index))) "yaw")))))
        (:then_6
          (bind _val_7 (CallFunction|GetValue (.Value (Utilities|Map|Find (.Value (Class|EjsonValue|JsonasObject (Utilities|Array|Get(acopy) (.Value (Class|EjsonValue|JsonasArray (Variables|Default|GetTmpLocations))) _array_index))) "vx")))))
        (:then_7
          (bind _val_8 (CallFunction|GetValue (.Value (Utilities|Map|Find (.Value (Class|EjsonValue|JsonasObject (Utilities|Array|Get(acopy) (.Value (Class|EjsonValue|JsonasArray (Variables|Default|GetTmpLocations))) _array_index))) "vy")))))
        (:then_8
          (bind _val_9 (CallFunction|GetValue (.Value (Utilities|Map|Find (.Value (Class|EjsonValue|JsonasObject (Utilities|Array|Get(acopy) (.Value (Class|EjsonValue|JsonasArray (Variables|Default|GetTmpLocations))) _array_index))) "vz")))))
        (:then_9
          (Utilities|Map|Add (Variables|Default|GetProxyCharacters) (.Value (Class|EjsonValue|JsonasString (.Value (Utilities|Map|Find (.Value (Class|EjsonValue|JsonasObject (Utilities|Array|Get(acopy) (.Value (Class|EjsonValue|JsonasArray (Variables|Default|GetTmpLocations))) _array_index))) "username")))) (Utilities|Struct|MakeSTRUCT_ProxyPlayer (.Value (Class|EjsonValue|JsonasString (.Value (Utilities|Map|Find (.Value (Class|EjsonValue|JsonasObject (Utilities|Array|Get(acopy) (.Value (Class|EjsonValue|JsonasArray (Variables|Default|GetTmpLocations))) _array_index))) "username")))) (Math|Vector|MakeVector _val _val_2 _val_3) (Math|Rotator|MakeRotator _val_4 _val_5 _val_6) (Math|Vector|MakeVector _val_7 _val_8 _val_9))))))
    (CallFunction|UpdateProxyLocation)))

(event Custom|FaceMouseDirection
  (params (DeltaSeconds :type Float%20%28single-precision%29))
  (bind _cachedhero (Variables|Default|GetCachedHero))
  ;[1 1 1] Input
  ;;[1 0.6917 0.6297] rotate
  (Utilities|IsValid _cachedhero
    (:Is%20Valid
      (Pawn|SetControlRotation (Math|Interpolation|RInterpTo (Transformation|GetActorRotation _cachedhero) (Variables|Default|GetMouseDirection) DeltaSeconds 1e+01)))))

(event Custom|UpdateProxyLocation
  (bind _outactors (Actor|GetAllActorsOfClass "/Game/Blueprint/DemoBP/BP_DemoBPProxyCharacter.BP_DemoBPProxyCharacter_C"))
  (for _array_element _outactors
    (if (.ReturnValue (Utilities|Map|Find (Variables|Default|GetProxyCharacters) (Variables|/Game/Blueprint/DemoBP/BP_DemoBPProxyCharacter.BP_DemoBPProxyCharacter_C|GetUsername _array_element)))
      (Variables|/Game/Blueprint/DemoBP/BP_DemoBPProxyCharacter.BP_DemoBPProxyCharacter_C|SetCurrentLocation _array_element (Math|Transform|MakeTransform (.Loction (Utilities|Struct|BreakSTRUCT_ProxyPlayer (.Value (Utilities|Map|Find (Variables|Default|GetProxyCharacters) (Variables|/Game/Blueprint/DemoBP/BP_DemoBPProxyCharacter.BP_DemoBPProxyCharacter_C|GetUsername _array_element))))) (.Rotation (Utilities|Struct|BreakSTRUCT_ProxyPlayer (.Value (Utilities|Map|Find (Variables|Default|GetProxyCharacters) (Variables|/Game/Blueprint/DemoBP/BP_DemoBPProxyCharacter.BP_DemoBPProxyCharacter_C|GetUsername _array_element))))) "1,1,1"))
      (Variables|/Script/Engine.MovementComponent|SetVelocity (Pawn|GetMovementComponent _array_element) (.Velocity (Utilities|Struct|BreakSTRUCT_ProxyPlayer (.Value (Utilities|Map|Find (Variables|Default|GetProxyCharacters) (Variables|/Game/Blueprint/DemoBP/BP_DemoBPProxyCharacter.BP_DemoBPProxyCharacter_C|GetUsername _array_element)))))))))

(event Custom|onTimeDo
  (Utilities|FlowControl|Sequence
    (:then_0
      (Variables|Default|SetbConnected (Variables|/Game/Blueprint/DemoBP/BP_DemoBPGameInstance.BP_DemoBPGameInstance_C|GetbConnected (Variables|Default|GetCachedGameInstance))))
    (:then_1
      (if (Variables|Default|GetbConnected)
        (Variables|Default|SetbOnTime true)))))

(event Custom|InitNetwork
  (bind _cachedhero (Variables|Default|GetCachedHero))
  (bind _returnvalue (Transformation|GetActorLocation _cachedhero))
  (bind _returnvalue_2 (Transformation|GetActorRotation _cachedhero))
  (bind _charactermovement (Variables|/Script/Engine.Character|GetCharacterMovement _cachedhero))
  (bind _returnvalue_3 (Pawn|Components|CharacterMovement|GetLastUpdateVelocity _charactermovement))
  (bind _asbp_demo_bpgame_instance (Utilities|Casting|CastToBP_DemoBPGameInstance (Game|GetGameInstance)))
  (bind _output_get (Variables|Default|SetCachedGameInstance _asbp_demo_bpgame_instance))
  (Utilities|IsValid (Variables|/Game/Blueprint/DemoBP/BP_DemoBPGameInstance.BP_DemoBPGameInstance_C|GetJsonRpcClient _output_get)
    (:Is%20Valid
      (Variables|Default|SetCached%20Json%20Rpc%20Client (Variables|/Game/Blueprint/DemoBP/BP_DemoBPGameInstance.BP_DemoBPGameInstance_C|GetJsonRpcClient _output_get))
      (Variables|Default|SetUpdateLocationReq (Class|EjsonValue|MakeJsonObject (Utilities|Map|MakeMap "username" (Class|EjsonValue|GetFieldValue (Variables|/Game/Blueprint/DemoBP/BP_DemoBPGameInstance.BP_DemoBPGameInstance_C|GetCachedUserInfo (Variables|Default|GetCachedGameInstance)) "username") "x" (Class|EjsonValue|MakeJsonNumber (.x _returnvalue)) "y" (Class|EjsonValue|MakeJsonNumber (.y _returnvalue)) "z" (Class|EjsonValue|MakeJsonNumber (.z _returnvalue)) "roll" (Class|EjsonValue|MakeJsonNumber (.roll _returnvalue_2)) "pitch" (Class|EjsonValue|MakeJsonNumber (.pitch _returnvalue_2)) "yaw" (Class|EjsonValue|MakeJsonNumber (.yaw _returnvalue_2)) "vx" (Class|EjsonValue|MakeJsonNumber (.x _returnvalue_3)) "vy" (Class|EjsonValue|MakeJsonNumber (.y _returnvalue_3)) "vz" (Class|EjsonValue|MakeJsonNumber (.z _returnvalue_3)))))
      (Utilities|Time|SetTimerbyEvent (EventDispatchers|CreateEvent :!event Custom|onTimeDo) 0.03 true))))

(event Custom|InitAllComponents
  ;[1 1 1] init all components
  ;;[1 0.6917 0.6297] mouse
  (Utilities|FlowControl|Sequence
    (:then_0
      (Variables|Default|SetbShowMouseCursor true))
    (:then_1
      (Variables|Default|SetbEnableClickEvents true))
    (:then_2
      (Input|SetInputModeGameandUI self 0 "DoNotLock" false))))

(event EventPossess
  (params (PossessedPawn :type Pawn%20Object%20Reference))
  (bind _asbp_demo_bphero_character (Utilities|Casting|CastToBP_DemoBPHeroCharacter PossessedPawn))
  (Variables|Default|SetCachedHero _asbp_demo_bphero_character))

(event EventBeginPlay
  (CallFunction|InitAllComponents)
  (CallFunction|InitNetWork))

(event EventTick
  (params (DeltaSeconds :type Float%20%28single-precision%29))
  (Utilities|FlowControl|Sequence
    (:then_0
      (CallFunction|SetMouseDirection))
    (:then_1
      (CallFunction|FaceMouseDirection DeltaSeconds))
    (:then_2
      (if (and (Variables|Default|GetbOnTime) (Variables|Default|GetbCanRequest))
        (Utilities|FillLocationReq
          (:Done
            (Class|ERpcConnection|Request (Variables|Default|GetCached%20Json%20Rpc%20Client) "UpdateLocation" (Class|EjsonValue|ToString (Variables|Default|GetUpdateLocationReq) false) (EventDispatchers|CreateEvent :!event Custom|OnUpdateLocation) 10)
            (Variables|Default|SetbCanRequest false)
            (Variables|Default|SetbOnTime false)))))))

(event Input|AxisEvents|InputAxisGoForward
  (params (AxisValue :type Float%20%28single-precision%29))
  ;[1 1 1] Input
  ;;[1 0.6917 0.6297] location
  (if (and (!= AxisValue 0.0) (Utilities|IsValid (Variables|Default|GetCachedHero)))
    (Pawn|Input|AddMovementInput (Variables|Default|GetCachedHero) (Math|Vector|MakeVector 1.0 0.0 0.0) AxisValue false)))

(event Input|AxisEvents|InputAxisGoBack
  (params (AxisValue :type Float%20%28single-precision%29))
  ;[1 1 1] Input
  ;;[1 0.6917 0.6297] location
  (if (and (!= AxisValue 0.0) (Utilities|IsValid (Variables|Default|GetCachedHero)))
    (Pawn|Input|AddMovementInput (Variables|Default|GetCachedHero) (Math|Vector|MakeVector 1.0 0.0 0.0) AxisValue false)))

(event Input|AxisEvents|InputAxisGoLeft
  (params (AxisValue :type Float%20%28single-precision%29))
  ;[1 1 1] Input
  ;;[1 0.6917 0.6297] location
  (if (and (!= AxisValue 0.0) (Utilities|IsValid (Variables|Default|GetCachedHero)))
    (Pawn|Input|AddMovementInput (Variables|Default|GetCachedHero) (Math|Vector|MakeVector 0.0 1.0 0.0) AxisValue false)))

(event Input|AxisEvents|InputAxisGoRight
  (params (AxisValue :type Float%20%28single-precision%29))
  ;[1 1 1] Input
  ;;[1 0.6917 0.6297] location
  (if (and (!= AxisValue 0.0) (Utilities|IsValid (Variables|Default|GetCachedHero)))
    (Pawn|Input|AddMovementInput (Variables|Default|GetCachedHero) (Math|Vector|MakeVector 0.0 1.0 0.0) AxisValue false)))

(fn ConstructionScript)

(fn GetValue
  (params (JsonVal :type Ejson%20Value%20Object%20Reference))
  (Utilities|IsValid JsonVal
    (:Is%20Valid
      (return (.Value (Class|EjsonValue|JsonasNumber JsonVal))))
    (:Is%20Not%20Valid
      (return 0.0))))