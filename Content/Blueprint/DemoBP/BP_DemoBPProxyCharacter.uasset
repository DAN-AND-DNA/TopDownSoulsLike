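; BP_DemoBPProxyCharacter is a proxy character that smoothly follows a target transform, with events that track its connected state.
; On BeginPlay it configures itself in code: capsule size, skeletal mesh, anim class, proxy material and movement, and stays tickable while paused.
; Each Tick interpolates location and rotation toward CurrentLocation, which is not set in these graphs, and teleports the actor there.
; An unconnected velocity-based move is left unused.
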(event Custom|InitAllComponents
  (bind _capsulecomponent (Variables|Default|GetCapsuleComponent))
  (bind _mesh (Variables|Character|GetMesh))
  ;[1 1 1] Init components
  (Class|Actor|SetTickablewhenPaused true)
  ;;[1 0.6917 0.6297] capsule
  (Utilities|FlowControl|Sequence
    (:then_0
      (Components|Capsule|SetCapsuleHalfHeight _capsulecomponent 75.0 true))
    (:then_1
      (Components|Capsule|SetCapsuleRadius _capsulecomponent 1.0 true)
      ;;[1 0.6917 0.6297] mesh
      (Utilities|FlowControl|Sequence
        (:then_0
          (Class|SkinnedMeshComponent|SetSkeletalMesh _mesh "/Game/Blender/mc3.mc3_Body7" true))
        (:then_1
          (Transformation|SetRelativeTransform _mesh (Variables|Default|GetMeshTransform) false false))
        (:then_2
          (Class|SkeletalMeshComponent|SetAnimClass _mesh "/Game/Blueprint/DemoBP/ABP_DemoBP.ABP_DemoBP_C"))
        (:then_3
          (Rendering|Material|SetMaterial _mesh 0 "/Game/Materials/M_Proxy.M_Proxy")
          ;;[1 0.6917 0.6297] movement
          (Utilities|FlowControl|Sequence
            (:then_0
              (Variables|/Script/Engine.CharacterMovementComponent|SetbRequestedMoveUseAcceleration (Variables|Character|GetCharacterMovement) true))))))))

(event Custom|OnConnected
  (Variables|Default|SetbConnected true))

(event Custom|OnDisconnected
  (Variables|Default|SetbConnected false))

(event EventBeginPlay
  (CallFunction|InitAllComponents)
  (Development|PrintString "New online"))

(event EventTick
  (params (DeltaSeconds :type Float%20%28single-precision%29))
  (bind _returnvalue (Transformation|GetActorTransform))
  (bind _currentlocation (Variables|Default|GetCurrentLocation))
  (bind (_location _rotation) (Math|Transform|BreakTransform _currentlocation))
  (Transformation|SetActorLocationAndRotation (Math|Interpolation|VInterpTo (.location _returnvalue) _location DeltaSeconds 2e+01) (Math|Interpolation|RInterpTo (.rotation _returnvalue) _rotation DeltaSeconds 2e+01) false true))

(event EventPossessed
  (params (NewController :type Controller%20Object%20Reference)))

(fn ConstructionScript
  (|CallParentFunction))