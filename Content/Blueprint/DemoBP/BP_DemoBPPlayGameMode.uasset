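; BP_DemoBPPlayGameMode is a demo game mode Blueprint for the play session.
; On BeginPlay it casts the game instance to BP_DemoBPGameInstance and caches the reference.
; If that instance holds a valid CachedUserInfo, it prints the info as a string, so user data stored on the game instance is read when play starts.
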(event EventBeginPlay
  (|CallParentFunction)
  (bind _asbp_demo_bpgame_instance (Utilities|Casting|CastToBP_DemoBPGameInstance (Game|GetGameInstance)))
  (bind _output_get (Variables|Default|SetCachedGameInstance _asbp_demo_bpgame_instance))
  (Utilities|IsValid (Variables|/Game/Blueprint/DemoBP/BP_DemoBPGameInstance.BP_DemoBPGameInstance_C|GetCachedUserInfo _output_get)
    (:Is%20Valid
      (Development|PrintString (Class|EjsonValue|ToString (Variables|/Game/Blueprint/DemoBP/BP_DemoBPGameInstance.BP_DemoBPGameInstance_C|GetCachedUserInfo _output_get) false)))))

(event EventTick
  (params (DeltaSeconds :type Float%20%28single-precision%29))
  (|CallParentFunction DeltaSeconds) ; This node is disabled and will not be called.\nDrag off pins to build functionality.
)

(fn ConstructionScript
  (|CallParentFunction))